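; Gameplay ability for a melee attack that turns the avatar toward its combat target and plays its attack montage, both handled through CombatInterface.
; Once the montage starts, it waits for the Event.Montage.Attack.Melee gameplay event, then draws a debug sphere at the combat socket location; no damage is applied yet.
; The ability ends when the montage completes, is interrupted or is cancelled.
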(event Ability|EventActivateAbility
  (bind _returnvalue (Ability|GetAvatarActorfromActorInfo))
  (bind _ascombat_interface (Utilities|Casting|CastToCombatInterface _returnvalue))
  (bind _returnvalue_2 (Class|CombatInterface|GetAttackMontage _ascombat_interface))
  (bind _returnvalue_3 (Class|EnemyInterface|GetCombatTarget(Message) _returnvalue))
  (Class|CombatInterface|UpdateFacingVector _ascombat_interface (Transformation|GetActorLocation _returnvalue_3))
  (|PlayMontageandWaitProxy "None" _returnvalue_2 1.0 "None" true 1.0 0.0 false
    (:then
      (Ability|Tasks|WaitGameplayEvent "(TagName=\"Event.Montage.Attack.Melee\")" 0
        (:EventReceived
          (bind _returnvalue_4 (Class|CombatInterface|GetCombatSocketLocation(Message) (Ability|GetAvatarActorfromActorInfo)))
          (Rendering|Debug|DrawDebugSphere _returnvalue_4 1e+01 12 "(R=1.000000,G=0.000000,B=0.096302,A=1.000000)" 1.0))))
    (:OnCompleted
      (Ability|EndAbility :!label _label))
    (:OnInterrupted
      (goto _label))
    (:OnCancelled
      (goto _label))))

(event Ability|EventOnEndAbility
  (params (bWasCancelled :type Boolean)))