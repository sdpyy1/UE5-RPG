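; Ranged attack gameplay ability that turns the avatar toward its combat target and fires a projectile at it.
; Combat interface calls on the avatar supply the target and attack montages, and a random tagged montage is played.
; A gameplay event matching that montage's tag spawns the projectile at the target's current location and ends the ability.
; Montage completion, interruption or cancellation also ends it.
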(event Ability|EventActivateAbility
  (bind _returnvalue (Ability|GetAvatarActorfromActorInfo))
  (bind _returnvalue_2 (Ability|GetAvatarActorfromActorInfo))
  ;[0.15 0.15 0.15 0.5] 获取敌人位置、调整攻击角度、获取攻击蒙太奇
  (Class|CombatInterface|GetCombatSocketLocation(Message) _returnvalue (Variables|Default|GetMontage%20Tag))
  (bind _returnvalue_3 (Class|EnemyInterface|GetCombatTarget(Message) _returnvalue))
  (Class|CombatInterface|UpdateFacingVector(Message) _returnvalue (Transformation|GetActorLocation _returnvalue_3))
  (bind _returnvalue_4 (Class|CombatInterface|GetAttackMontages(Message) _returnvalue))
  (bind _returnvalue_5 (Class|AuraAbilitySystemLibrary|GetRandomTaggedMontage _returnvalue_4))
  (|PlayMontageandWaitProxy "None" (.Montage (Utilities|Struct|BreakTaggedMontage _returnvalue_5)) 1.0 "None" false 1.0 0.0 false
    (:then
      (Ability|Tasks|WaitGameplayEvent (.MontageTag (Utilities|Struct|BreakTaggedMontage _returnvalue_5)) 0
        (:EventReceived
          (bind _returnvalue_6 (Class|EnemyInterface|GetCombatTarget(Message) _returnvalue_2))
          (Class|AuraRangeAttackAbility|SpawnProjectile _returnvalue_2 (Transformation|GetActorLocation _returnvalue_6))
          (Ability|EndAbility))))
    (:OnCompleted
      (Ability|EndAbility :!label _label))
    (:OnInterrupted
      (goto _label))
    (:OnCancelled
      (goto _label))))

(event Ability|EventOnEndAbility
  (params (bWasCancelled :type Boolean)))