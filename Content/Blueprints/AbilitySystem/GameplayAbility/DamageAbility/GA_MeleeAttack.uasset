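; Melee attack gameplay ability that turns the avatar toward its combat target and damages actors tagged "player".
; It plays a random tagged montage and waits for that montage's gameplay event to sphere-query live players around the matching combat socket.
; Each hit spawns the victim's blood effect and applies damage, with one impact sound if anything was hit.
; The ability ends after the hit check or when the montage completes, is interrupted or is cancelled.
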(event Ability|EventActivateAbility
  (bind _returnvalue (Ability|GetAvatarActorfromActorInfo))
  (bind _returnvalue_2 (Ability|GetAvatarActorfromActorInfo))
  (Utilities|FlowControl|Sequence
    (:then_0
      ;[0.15 0.15 0.15 0.5] 朝向敌人
      (bind _returnvalue_3 (Class|EnemyInterface|GetCombatTarget(Message) _returnvalue))
      (bind _ascombat_interface (Utilities|Casting|CastToCombatInterface _returnvalue))
      (Class|CombatInterface|UpdateFacingVector _ascombat_interface (Transformation|GetActorLocation _returnvalue_3)))
    (:then_1
      ;[0.15 0.15 0.15 0.5] 获取一个攻击蒙太奇
      (bind _returnvalue_4 (Class|CombatInterface|GetAttackMontages(Message) (Ability|GetAvatarActorfromActorInfo)))
      (bind _returnvalue_5 (Class|AuraAbilitySystemLibrary|GetRandomTaggedMontage _returnvalue_4))
      (|PlayMontageandWaitProxy "None" (.Montage (Utilities|Struct|BreakTaggedMontage _returnvalue_5)) 1.0 "None" false 1.0 0.0 false
        (:then
          (Ability|Tasks|WaitGameplayEvent (.MontageTag (Utilities|Struct|BreakTaggedMontage _returnvalue_5)) 0
            (:EventReceived
              (bind _returnvalue_6 (Class|CombatInterface|GetCombatSocketLocation(Message) (Ability|GetAvatarActorfromActorInfo) (.MontageTag (Utilities|Struct|BreakTaggedMontage _returnvalue_5))))
              ;[0.15 0.15 0.15 0.5] 查询攻击击中，播放声音、添加特效、造成伤害、结束能力
              (bind _outoverlappingactors (Class|AuraAbilitySystemLibrary|GetLivePlayerWithinRadius _returnvalue_2 (Utilities|Array|MakeArray _returnvalue_2) _returnvalue_6 2e+02))
              (for _array_element _outoverlappingactors
                (if (Actor|ActorHasTag _array_element "player")
                  (bind _returnvalue_7 (Class|CombatInterface|GetBloodEffect(Message) _array_element))
                  (Niagara|SpawnSystematLocation _returnvalue_7 _returnvalue_6)
                  (Class|DamageGameplayAbility|CauseDamage _array_element)
                  (Variables|Default|SethasTargetHit true)))
              (if (Variables|Default|GethasTargetHit)
                (Audio|PlaySoundatLocation (.HitSound (Utilities|Struct|BreakTaggedMontage _returnvalue_5)) _returnvalue_6 "0, 0, 0" 1.0 1.0 0.0 0 0 0 0))
              (Ability|EndAbility))))
        (:OnCompleted
          (Ability|EndAbility :!label _label))
        (:OnInterrupted
          (goto _label))
        (:OnCancelled
          (goto _label))))
    (:then_2
      (Variables|Default|SethasTargetHit false))))

(event Ability|EventOnEndAbility
  (params (bWasCancelled :type Boolean)))