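; GA_FireBolt is the gameplay ability that casts a Fire Bolt projectile toward the point under the mouse.
; On activation it reads the mouse target location through target data and turns the avatar toward it via CombatInterface.
; It then plays the cast montage and waits for the Event.Montage.FireBolt gameplay event, so the montage times the shot.
; That event spawns the projectile at the stored target and ends the ability.
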(event Ability|EventActivateAbility
  (bind _datahandle (|GetTargetDataUnderMouse)
    (:then
      (Variables|Default|SetTargetLocation (.Location (Collision|BreakHitResult (Ability|TargetData|GetHitResultfromTargetData _datahandle))))
      (bind _ascombat_interface (Utilities|Casting|CastToCombatInterface (Ability|GetAvatarActorfromActorInfo)))
      (Class|CombatInterface|UpdateFacingVector _ascombat_interface (Variables|Default|GetTargetLocation))
      (|PlayMontageandWaitProxy "None" "/Game/Assets/Characters/Aura/Animations/Abilities/AM_Cast_FireBolt.AM_Cast_FireBolt" 1.0 "None" true 1.0 0.0 false
        (:then
          (Ability|Tasks|WaitGameplayEvent "(TagName=\"Event.Montage.FireBolt\")" 0
            (:EventReceived
              (Class|AuraProjectileSpellAbility|SpawnProjectile (Variables|Default|GetTargetLocation))
              (Ability|EndAbility))))))))

(event Ability|EventOnEndAbility
  (params (bWasCancelled :type Boolean)))